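; BP_Portail is a gate that the player opens and closes by pressing ActionTouch while inside its trigger box.
; Box overlap enables input and a Gate node for the first-person character, whose Diego flag must be set, otherwise a message prints.
; A FlipFlop plays or reverses the TempOuveture timeline to yaw PortailDieg.
; The timeline track feeds the Lerp's A input rather than Alpha; a vertical-slide branch is unconnected.
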(event `InputAction|ActionTouch`
  (params (Key :type "Key Structure"))
  (:`Pressed`
    (if (`/Game/FirstPerson/Blueprints/BP_FirstPersonCharacter.Diego` (stale `self.Box.OnComponentBeginOverlap` _asbp_first_person_character))
      (`/Engine/EditorBlueprintResources/StandardMacros.Gate` true :!label _label
        (:`Exit`
          (`/Engine/EditorBlueprintResources/StandardMacros.FlipFlop`
            (:`A`
              (bind (_direction _trackporte) (`Timeline|Temp ouveture` :!label _label_2)
                (:`Update`
                  (`SceneComponent.K2_SetRelativeRotation` (`self.Portail_Dieg`) (`KismetMathLibrary.MakeRotator` 0.0 0.0 (`KismetMathLibrary.Lerp` _trackporte (`self.PositionNeutre`) (`self.PositionOuvert`))) false false))))
            (:`B`
              (goto _label_2 :!via `Reverse`)))))
      (else
        (`KismetSystemLibrary.PrintString` "Poccède pas la valise ^^")))))

(event `self.Box.OnComponentBeginOverlap`
  (params (OverlappedComponent :type "PrimitiveComponent Object Reference") (OtherActor :type "Actor Object Reference") (OtherComp :type "PrimitiveComponent Object Reference") (OtherBodyIndex :type Integer) (bFromSweep :type Boolean) (SweepResult :type "HitResult Structure (by ref)"))
  (bind _asbp_first_person_character (cast `/Game/FirstPerson/Blueprints/BP_FirstPersonCharacter` OtherActor))
  (`self.EnableInput` (`GameplayStatics.GetPlayerController` 0))
  (goto _label :!via `Open`))

(event `self.Box.OnComponentEndOverlap`
  (params (OverlappedComponent :type "PrimitiveComponent Object Reference") (OtherActor :type "Actor Object Reference") (OtherComp :type "PrimitiveComponent Object Reference") (OtherBodyIndex :type Integer))
  (cast `/Game/FirstPerson/Blueprints/BP_FirstPersonCharacter` OtherActor)
  (`self.DisableInput` (`GameplayStatics.GetPlayerController` 0))
  (goto _label :!via `Close`))

(fn `UserConstructionScript`)